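; Base projectile actor for weapons that damages whatever it hits and then removes itself.
; On Hit it stores the other actor, then runs ApplyDamageByProjectile followed by OnEndOfHit, which destroys the projectile.
; Damage comes from the current damage of its BP_WeaponBase owner, uses the BP_DamageObject damage type and credits the weapon's owner as causer.
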(event EventBeginPlay)

(event Collision|EventActorBeginOverlap
  (params (OtherActor :type Actor%20Object%20Reference)))

(event EventTick
  (params (DeltaSeconds :type Float%20%28single-precision%29)))

(event Collision|EventHit
  (params (MyComp :type Primitive%20Component%20Object%20Reference) (Other :type Actor%20Object%20Reference) (OtherComp :type Primitive%20Component%20Object%20Reference) (bSelfMoved :type Boolean) (HitLocation :type Vector :default "0, 0, 0") (HitNormal :type Vector :default "0, 0, 0") (NormalImpulse :type Vector :default "0, 0, 0") (Hit :type Hit%20Result%20Structure%20%28by%20ref%29))
  (Variables|Default|SetOther Other)
  (Utilities|FlowControl|Sequence
    (:then_0
      (CallFunction|ApplyDamagebyProjectile))
    (:then_1
      (CallFunction|OnEndOfHit))))

(fn ConstructionScript)

(fn OnEndOfHit
  (Actor|DestroyActor))

(fn ApplyDamagebyProjectile
  (bind _asbp_weapon_base (Utilities|Casting|CastToBP_WeaponBase (Components|GetOwner)))
  (Game|Damage|ApplyDamage (Variables|Default|GetOther) (Math|Conversions|ToFloat(Integer) (Variables|/Game/Blueprints/Weapons/BP_WeaponBase.BP_WeaponBase_C|GetDamageCurrent _asbp_weapon_base)) 0 (Components|GetOwner (Components|GetOwner)) "/Game/Blueprints/Objects/BP_DamageObject.BP_DamageObject_C"))